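; BP_Enemy is a short-lived enemy actor that expires after 20 seconds and reacts to overlaps on its collision mesh.
; A BP_Projectile hit destroys both actors and increments the Score on the BP_Player found via GetActorOfClass.
; A BP_Player hit destroys the enemy, decrements player Health and plays a world camera shake at the player's location.
; When Health reaches zero or below, it calls the player's DisplayRestart.
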(event OnComponentBeginOverlap(CollisionMesh)
  (params (OverlappedComponent :type Primitive%20Component%20Object%20Reference) (OtherActor :type Actor%20Object%20Reference) (OtherComp :type Primitive%20Component%20Object%20Reference) (OtherBodyIndex :type Integer) (bFromSweep :type Boolean) (SweepResult :type Hit%20Result%20Structure%20%28by%20ref%29))
  (Utilities|FlowControl|Sequence
    (:then_0
      (bind _asbp_projectile (Utilities|Casting|CastToBP_Projectile OtherActor))
      (Utilities|FlowControl|Sequence
        (:then_0
          (Actor|DestroyActor :!label _label))
        (:then_1
          (Actor|DestroyActor _asbp_projectile))
        (:then_2
          (bind _returnvalue (Actor|GetActorOfClass "/Game/InfiniteMatrix/Blueprints/BP_Player.BP_Player_C"))
          (bind _result (Math|Float|IncrementFloat (Variables|/Game/InfiniteMatrix/Blueprints/BP_Player.BP_Player_C|GetScore _returnvalue))
            (:%20%20
              (Variables|/Game/InfiniteMatrix/Blueprints/BP_Player.BP_Player_C|SetScore _returnvalue _result))))))
    (:then_1
      (bind _asbp_player (Utilities|Casting|CastToBP_Player OtherActor))
      (Utilities|FlowControl|Sequence
        (:then_0
          (goto _label))
        (:then_1
          (bind _result_2 (Math|Float|DecrementFloat (Variables|/Game/InfiniteMatrix/Blueprints/BP_Player.BP_Player_C|GetHealth _asbp_player))
            (:%20%20
              (bind _output_get (Variables|/Game/InfiniteMatrix/Blueprints/BP_Player.BP_Player_C|SetHealth _asbp_player _result_2))
              (if (<= _output_get 0.0)
                (Default|DisplayRestart _asbp_player)))))
        (:then_2
          (Camera|PlayWorldCameraShake "/Game/InfiniteMatrix/Blueprints/BP_Camera_Shake.BP_Camera_Shake_C" (Transformation|GetActorLocation _asbp_player) 0.0 5e+02))))))

(event EventBeginPlay
  (Actor|SetLifeSpan 2e+01))

(event Collision|EventActorBeginOverlap
  (params (OtherActor :type Actor%20Object%20Reference)))

(event EventTick
  (params (DeltaSeconds :type Float%20%28single-precision%29)))

(fn ConstructionScript)